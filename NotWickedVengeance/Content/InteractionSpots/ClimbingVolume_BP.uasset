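; Climbing spot (a tree, per the graph comments) that spawns a random mesh actor and lets the player climb it.
; Its volume toggles input; holding Interact loops on a short Delay, setting Flying, pushing upward and orienting the character mesh from its HitResult.
; Release or leaving the volume restores Walking and mesh rotation on the next check.
; An overlap passing an AIController cast swaps the spawned mesh for a random destroyed variant.
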(event `self.Climbing Volume.OnComponentBeginOverlap`
  (params (OverlappedComponent :type "PrimitiveComponent Object Reference") (OtherActor :type "Actor Object Reference") (OtherComp :type "PrimitiveComponent Object Reference") (OtherBodyIndex :type Integer) (bFromSweep :type Boolean) (SweepResult :type "HitResult Structure (by ref)"))
  ;[1 1 1] Check Overlap
  (cast `/Game/ThirdPersonBP/Blueprints/ThirdPersonCharacter` OtherActor)
  (`self.EnableInput` (`GameplayStatics.GetPlayerController` 0))
  (set `self.IsClimbing` true))

(event `self.Climbing Volume.OnComponentEndOverlap`
  (params (OverlappedComponent :type "PrimitiveComponent Object Reference") (OtherActor :type "Actor Object Reference") (OtherComp :type "PrimitiveComponent Object Reference") (OtherBodyIndex :type Integer))
  ;[1 1 1] Check Overlap
  (cast `/Game/ThirdPersonBP/Blueprints/ThirdPersonCharacter` OtherActor)
  (`self.DisableInput` (`GameplayStatics.GetPlayerController` 0))
  (set `self.IsClimbing` false))

(event `InputAction|Interact`
  (params (Key :type "Key Structure"))
  (bind _returnvalue (`GameplayStatics.GetPlayerCharacter` 0))
  (bind _returnvalue_2 (`GameplayStatics.GetPlayerCharacter` 0))
  (bind _returnvalue_3 (`GameplayStatics.GetPlayerPawn` 0))
  (bind _asthird_person_character (cast `/Game/ThirdPersonBP/Blueprints/ThirdPersonCharacter` _returnvalue_2 :!pure true))
  (bind _hitresult (`/Game/ThirdPersonBP/Blueprints/ThirdPersonCharacter.HitResult` _asthird_person_character))
  ;[1 1 1] Interact to Climb Around Tree
  (:`Pressed`
    (if (`self.IsClimbing`) :!label _label
      (if (`PlayerController.IsInputKeyDown` (`GameplayStatics.GetPlayerController` 0) Key)
        (`CharacterMovementComponent.SetMovementMode` (`Character.CharacterMovement` _returnvalue_2) "MOVE_Flying" 0)
        (`Pawn.AddMovementInput` _returnvalue_3 (`self.GetActorUpVector` _returnvalue_3) 10.0 false)
        (`SceneComponent.K2_SetWorldRotation` (`Character.Mesh` _asthird_person_character) (`KismetMathLibrary.MakeRotationFromAxes` _hitresult _hitresult) false false)
        (`KismetSystemLibrary.Delay` 0.2)
        (goto _label)
        (else
          _)))
    (`CharacterMovementComponent.SetMovementMode` (`Character.CharacterMovement` _returnvalue) "MOVE_Walking" 0)
    (`SceneComponent.K2_SetRelativeRotation` (`Character.Mesh` (cast `/Game/ThirdPersonBP/Blueprints/ThirdPersonCharacter` _returnvalue :!pure true)) (`KismetMathLibrary.MakeRotator` 0.0 0.0 -90.0) false false)))

(event `self.ReceiveBeginPlay`
  (bind _random_mesh_actor (`self.Random Mesh Actor`))
  ;[1 1 1] Spawn Random Mesh
  (bind _returnvalue (`|SpawnActorFromClass` (`|GetArrayItem` _random_mesh_actor (`KismetMathLibrary.RandomIntegerInRange` 0 (`KismetArrayLibrary.Array_LastIndex` _random_mesh_actor))) (`KismetMathLibrary.Conv_VectorToTransform` (`SceneComponent.K2_GetComponentLocation` (`self.DefaultSceneRoot`))) "Undefined" "OverrideRootScale" null null))
  (set `self.Created Mesh` _returnvalue))

(event `self.MonsterCollisionCheck.OnComponentBeginOverlap`
  (params (OverlappedComponent :type "PrimitiveComponent Object Reference") (OtherActor :type "Actor Object Reference") (OtherComp :type "PrimitiveComponent Object Reference") (OtherBodyIndex :type Integer) (bFromSweep :type Boolean) (SweepResult :type "HitResult Structure (by ref)"))
  (bind _destroyed_mesh_array (`self.Destroyed Mesh Array`))
  ;[1 1 1] If Monster Runs Over Mesh Destroy It
  (cast `AIController` OtherActor)
  (`self.K2_DestroyActor` (`self.Created Mesh`))
  (`|SpawnActorFromClass` (`|GetArrayItem` _destroyed_mesh_array (`KismetMathLibrary.RandomIntegerInRange` 0 (`KismetArrayLibrary.Array_LastIndex` _destroyed_mesh_array))) (`KismetMathLibrary.Conv_VectorToTransform` (`SceneComponent.K2_GetComponentLocation` (`self.DefaultSceneRoot`))) "Undefined" "OverrideRootScale" null null))

(fn `UserConstructionScript`)